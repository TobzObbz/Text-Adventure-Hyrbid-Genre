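; Helper functions for a room-based text adventure with chests, health potions and zombie combat, played through a first-person character.
; CommandCommit parses typed text into commands, using long or short phrases by stage.
; CheckMovement validates exits and zombie blocking, then MoveRooms teleports the player and minimap, while RoomWalk derives room IDs from position.
; Description functions append event text, reading per-room state from Chest_BP and Zombie_BP found via GetActorOfClass.
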(fn ChestDescription
  (params (Room%20ID :type Integer) (Description :type String) (Command :type Command%20Enum :default "NewEnumerator0") (Health%20Potions :type Integer) (Chest%20Description%20Displayed? :type Boolean))
  ;[1 1 1] Chest
  (bind _returnvalue (Actor|GetActorOfClass 0 "/Game/Blueprints/Chest_BP.Chest_BP_C"))
  (bind _values (Utilities|Map|Values (Variables|/Game/Blueprints/Chest_BP.Chest_BP_C|GetChest_0 _returnvalue)))
  (if (and (Utilities|Array|Get(acopy) _values Room%20ID) (Utilities|Enum|Equal(Enum) Command "NewEnumerator4"))
    (bind _result (Math|Integer|IncrementInt Health%20Potions)
      (:%20%20
        (return (Utilities|String|Append Description " 
> You found a health potion, it has been added to your inventory ") true _result false)))
    (elif (Utilities|Array|Get(acopy) _values Room%20ID)
      (if Chest%20Description%20Displayed?
        (return Description false Health%20Potions true)
        (else
          (return (Utilities|String|Append Description " 
> There is also a chest in the room ") false Health%20Potions true)))
      (else
        (return Description false Health%20Potions false)))))

(fn ZombieDescription
  (params (Room%20ID :type Integer) (Description :type String))
  (bind _returnvalue (Actor|GetActorOfClass 0 "/Game/Blueprints/Zombie_BP.Zombie_BP_C"))
  (bind _values (Utilities|Map|Values (Variables|/Game/Blueprints/Zombie_BP.Zombie_BP_C|GetZombie _returnvalue)))
  (if (Utilities|Array|Get(acopy) _values Room%20ID)
    (return (Utilities|String|Append Description " 
> A zombie stands in your way, blocking the exit "))
    (else
      (return Description))))

(fn DrinkPotion
  (params (Description :type String) (Command :type Command%20Enum :default "NewEnumerator0") (Health%20Potions :type Integer))
  (bind _returnvalue (Game|GetPlayerCharacter 0))
  (bind _asbp_first_person_character (Utilities|Casting|CastToBP_FirstPersonCharacter _returnvalue))
  ;[1 1 1] Drink Health Potion
  (if (and (> Health%20Potions 0) (Utilities|Enum|Equal(Enum) Command "NewEnumerator5"))
    (bind _result (Math|Integer|DecrementInt Health%20Potions)
      (:%20%20
        (bind _returnvalue_2 (UserInterface|CreateWidget "/Game/UI/TextAdventure_UI.TextAdventure_UI_C"))
        (if (Variables|/Game/UI/TextAdventure_UI.TextAdventure_UI_C|GetHealth%20Bar _returnvalue_2)
          (return "" _result)
          (elif (>= (Variables|/Game/FirstPerson/Blueprints/BP_FirstPersonCharacter.BP_FirstPersonCharacter_C|GetHealth _asbp_first_person_character) 0.0)
            (return (Utilities|String|Append Description " 
> You drink the health potion. You have  " (Utilities|String|ToString(Integer) (Math|Float|Round (Variables|/Game/FirstPerson/Blueprints/BP_FirstPersonCharacter.BP_FirstPersonCharacter_C|GetHealth _asbp_first_person_character))) "HP 
> You are at max health ") _result)
            (else
              (return (Utilities|String|Append Description " 
> You drink the health potion. You have " (Utilities|String|ToString(Integer) (Math|Float|Round (Variables|/Game/FirstPerson/Blueprints/BP_FirstPersonCharacter.BP_FirstPersonCharacter_C|GetHealth _asbp_first_person_character))) "HP") _result))))))
    (else
      (return Description Health%20Potions))))

(fn AttackZombie
  (params (Room%20ID :type Integer) (Description :type String) (Command :type Command%20Enum :default "NewEnumerator0"))
  ;[1 1 1] Attack Zombie
  (bind _returnvalue (Actor|GetActorOfClass 0 "/Game/Blueprints/Zombie_BP.Zombie_BP_C"))
  (bind _values (Utilities|Map|Values (Variables|/Game/Blueprints/Zombie_BP.Zombie_BP_C|GetZombie _returnvalue)))
  (if (and (Utilities|Array|Get(acopy) _values Room%20ID) (Utilities|Enum|Equal(Enum) Command "NewEnumerator6"))
    (bind _returnvalue_2 (Actor|GetActorOfClass 0 "/Game/Blueprints/Zombie_BP.Zombie_BP_C"))
    (if (Variables|/Game/Blueprints/Zombie_BP.Zombie_BP_C|GetZombie%20Dead? _returnvalue_2)
      (bind _output_get (Variables|/Game/Blueprints/Zombie_BP.Zombie_BP_C|SetZombie%20Dead? _returnvalue_2 true))
      (return (Utilities|String|Append Description " 
> You attacked for " (Utilities|String|ToString(Integer) (Variables|/Game/Blueprints/Zombie_BP.Zombie_BP_C|GetAttack%20Damage _returnvalue_2)) " HP " " 
> The zombie is dead ") (Utilities|String|Len Description) _output_get true)
      (else
        (return (Utilities|String|Append Description " 
> You attacked for " (Utilities|String|ToString(Integer) (Variables|/Game/Blueprints/Zombie_BP.Zombie_BP_C|GetAttack%20Damage _returnvalue_2)) " HP " " 
> The zombie is still standing ") (Utilities|String|Len Description) false true)))
    (else
      (return Description (Utilities|String|Len Description) false false))))

(fn ZombieAttack
  (params (Description :type String))
  ;[1 1 1] Zombie Attack
  (bind _returnvalue (Actor|GetActorOfClass 0 "/Game/Blueprints/Zombie_BP.Zombie_BP_C"))
  (if (Variables|/Game/Blueprints/Zombie_BP.Zombie_BP_C|GetZombie%20Punch _returnvalue)
    (bind _returnvalue_2 (Actor|GetActorOfClass 0 "/Game/Blueprints/Zombie_BP.Zombie_BP_C"))
    (Variables|/Game/Blueprints/Zombie_BP.Zombie_BP_C|SetZombie%20Punch _returnvalue_2 false)
    (return (Utilities|String|Append Description " 
> The zombie attacked you for " (Utilities|String|ToString(Integer) (Variables|/Game/Blueprints/Zombie_BP.Zombie_BP_C|GetZombie%20Damage _returnvalue)) "HP. You have " (Utilities|String|ToString(Integer) (Math|Float|Round (Variables|/Game/FirstPerson/Blueprints/BP_FirstPersonCharacter.BP_FirstPersonCharacter_C|GetHealth (.AsBP%20First%20Person%20Character (Utilities|Casting|CastToBP_FirstPersonCharacter (Game|GetPlayerCharacter 0)))))) "HP"))
    (else
      (return Description))))

(fn CommandCommit
  (params (Text :type String) (Stage :type Integer) (Room%20ID :type Integer) (Underscore%20Movement%20Timer :type Timer%20Handle%20Structure) (Health%20Potions :type Integer))
  (bind _returnvalue (Game|GetPlayerCharacter 0))
  (bind _asbp_first_person_character (Utilities|Casting|CastToBP_FirstPersonCharacter _returnvalue))
  ;[1 1 1] Movement Commands
  (Utilities|Time|ClearandInvalidateTimerbyHandle 0 Underscore%20Movement%20Timer)
  (if (or (and (Utilities|Enum|Equal(Enum) Text "Go North") (== Stage 1)) (and (Utilities|Enum|Equal(Enum) Text "N") (> Stage 1)))
    (bind _output_get (LocalVariables|SetCommand "NewEnumerator0"))
    (return _output_get true)
    (elif (or (and (Utilities|Enum|Equal(Enum) Text "Go East") (== Stage 1)) (and (Utilities|Enum|Equal(Enum) Text "E") (> Stage 1)))
      (bind _output_get_2 (LocalVariables|SetCommand "NewEnumerator1"))
      (return _output_get_2 true)
      (elif (or (and (Utilities|Enum|Equal(Enum) Text "Go South") (== Stage 1)) (and (Utilities|Enum|Equal(Enum) Text "S") (> Stage 1)))
        (bind _output_get_3 (LocalVariables|SetCommand "NewEnumerator2"))
        (return _output_get_3 true)
        (elif (or (and (Utilities|Enum|Equal(Enum) Text "Go West") (== Stage 1)) (and (Utilities|Enum|Equal(Enum) Text "W") (> Stage 1)))
          (bind _output_get_4 (LocalVariables|SetCommand "NewEnumerator3"))
          (return _output_get_4 true)
          (else
            ;[1 1 1] Utility Commands
            (bind _returnvalue_2 (Actor|GetActorOfClass 0 "/Game/Blueprints/Chest_BP.Chest_BP_C"))
            (bind _values (Utilities|Map|Values (Variables|/Game/Blueprints/Chest_BP.Chest_BP_C|GetChest_0 _returnvalue_2)))
            (if (and (Utilities|Array|Get(acopy) _values Room%20ID) (or (and (Utilities|Enum|Equal(Enum) Text "Use Chest") (== Stage 1)) (and (Utilities|Enum|Equal(Enum) Text "Chest") (> Stage 1))))
              (bind _output_get_5 (LocalVariables|SetCommand "NewEnumerator4"))
              (return _output_get_5 true)
              (elif (and (or (and (Utilities|Enum|Equal(Enum) Text "Use Health Potion") (== Stage 1)) (and (Utilities|Enum|Equal(Enum) Text "Health Potion") (> Stage 1))) (> Health%20Potions 0))
                (bind _output_get_6 (LocalVariables|SetCommand "NewEnumerator5"))
                (if (>= (+ (Variables|/Game/FirstPerson/Blueprints/BP_FirstPersonCharacter.BP_FirstPersonCharacter_C|GetHealth _asbp_first_person_character) 2e+01) 5e+01)
                  (Variables|/Game/FirstPerson/Blueprints/BP_FirstPersonCharacter.BP_FirstPersonCharacter_C|SetHealth _asbp_first_person_character 5e+01)
                  (return _output_get_6 true)
                  (else
                    (Variables|/Game/FirstPerson/Blueprints/BP_FirstPersonCharacter.BP_FirstPersonCharacter_C|SetHealth _asbp_first_person_character (Variables|/Game/FirstPerson/Blueprints/BP_FirstPersonCharacter.BP_FirstPersonCharacter_C|GetHealth _asbp_first_person_character))
                    (return _output_get_6 true)))
                (else
                  (bind _returnvalue_3 (Actor|GetActorOfClass 0 "/Game/Blueprints/Zombie_BP.Zombie_BP_C"))
                  (bind _values_2 (Utilities|Map|Values (Variables|/Game/Blueprints/Zombie_BP.Zombie_BP_C|GetZombie _returnvalue_3)))
                  (if (and (Utilities|Array|Get(acopy) _values_2 Room%20ID) (or (and (== Stage 1) (Utilities|Enum|Equal(Enum) Text "Attack Zombie")) (and (Utilities|Enum|Equal(Enum) Text "A") (> Stage 1))))
                    (bind _output_get_7 (LocalVariables|SetCommand "NewEnumerator6"))
                    (bind _returnvalue_4 (Actor|GetActorOfClass 0 "/Game/Blueprints/Zombie_BP.Zombie_BP_C"))
                    (Default|AttackZombie _returnvalue_4)
                    (Default|Attack (.AsBP%20First%20Person%20Character (Utilities|Casting|CastToBP_FirstPersonCharacter (Game|GetPlayerCharacter 0))))
                    (return _output_get_7 true)
                    (else
                      (return "NewEnumerator7" false))))))))))))

(fn CheckMovement
  (params (RoomID :type Integer) (Command :type Command%20Enum :default "NewEnumerator0"))
  (bind _values (Utilities|Map|Values (LocalVariables|GetAvailable%20Directions)))
  (bind _returnvalue (Actor|GetActorOfClass 0 "/Game/Blueprints/Zombie_BP.Zombie_BP_C"))
  (bind _values_2 (Utilities|Map|Values (Variables|/Game/Blueprints/Zombie_BP.Zombie_BP_C|GetZombie _returnvalue)))
  (if (or (and (not (Utilities|Array|Get(acopy) _values_2 RoomID)) (Utilities|Select :Index Command :NewEnumerator0 (Utilities|String|Contains (Utilities|Array|Get(acopy) _values RoomID) "N") :NewEnumerator1 (Utilities|String|Contains (Utilities|Array|Get(acopy) _values RoomID) "E") :NewEnumerator2 (Utilities|String|Contains (Utilities|Array|Get(acopy) _values RoomID) "S") :NewEnumerator3 (Utilities|String|Contains (Utilities|Array|Get(acopy) _values RoomID) "W") :NewEnumerator4 false :NewEnumerator5 false :NewEnumerator6 false :NewEnumerator7 false)) (== RoomID 13))
    (return true (Utilities|Select :Index Command :NewEnumerator0 (Math|Float|MakeLiteralFloat 1e+03) :NewEnumerator1 0.0 :NewEnumerator2 (Math|Float|MakeLiteralFloat -1e+03) :NewEnumerator3 0.0 :NewEnumerator4 0.0 :NewEnumerator5 0.0 :NewEnumerator6 0.0 :NewEnumerator7 0.0) (Utilities|Select :Index Command :NewEnumerator0 0.0 :NewEnumerator1 (Math|Float|MakeLiteralFloat 1e+03) :NewEnumerator2 0.0 :NewEnumerator3 (Math|Float|MakeLiteralFloat -1e+03) :NewEnumerator4 0.0 :NewEnumerator5 0.0 :NewEnumerator6 0.0 :NewEnumerator7 0.0))
    (else
      (return false 0.0 0.0))))

(fn MoveRooms
  (params (X :type Float%20%28double-precision%29) (Y :type Float%20%28double-precision%29) (Room%20ID :type Integer))
  ;[1 1 1] Work out what the new room ID will be and move in the right direction
  (LocalVariables|SetNew%20Location (+ (.Value (Utilities|Map|Find (LocalVariables|GetRoom%20Locations) Room%20ID)) (Math|Vector|MakeVector X Y 0.0)))
  (bind _values (Utilities|Map|Values (LocalVariables|GetRoom%20Locations)))
  (bind (_array_element _array_index) (Utilities|Array|ForEachLoopwithBreak _values :!label _label)
    (:LoopBody
      (if (Utilities|Operators|EqualEqual _array_element (LocalVariables|GetNew%20Location) 3e+02)
        (LocalVariables|SetNew%20Room%20ID _array_index)
        (bind _returnvalue (Actor|GetActorOfClass 0 "/Game/Blueprints/MiniMap_BP.MiniMap_BP_C"))
        (Transformation|SetWorldLocation (Variables|/Game/Blueprints/MiniMap_BP.MiniMap_BP_C|GetDefaultSceneRoot _returnvalue) (Math|Vector|MakeVector (.X (Math|Vector|BreakVector (LocalVariables|GetNew%20Location))) (.Y (Math|Vector|BreakVector (LocalVariables|GetNew%20Location))) 2.7e+03) false false)
        (Transformation|SetWorldLocation (Variables|/Script/Engine.Actor|GetRootComponent (Game|GetPlayerCharacter 0)) (Math|Vector|MakeVector (.X (Math|Vector|BreakVector (LocalVariables|GetNew%20Location))) (.Y (Math|Vector|BreakVector (LocalVariables|GetNew%20Location))) 125.0) false false)
        (LocalVariables|SetMovement%20Successful true)
        (goto _label Break)))
    (:Completed
      (bind _returnvalue_2 (Actor|GetActorOfClass 0 "/Game/Blueprints/Zombie_BP.Zombie_BP_C"))
      (Variables|/Game/Blueprints/Zombie_BP.Zombie_BP_C|SetZombie%20Dead? _returnvalue_2 false)
      (bind _returnvalue_3 (Actor|GetActorOfClass 0 "/Game/Blueprints/Door_BP.Door_BP_C"))
      (Default|OpenClose _returnvalue_3)
      (return (LocalVariables|GetNew%20Room%20ID)))))

(fn Movement?
  (params (Command :type Command%20Enum :default "NewEnumerator0"))
  (return (Math|Boolean|ORBoolean (Utilities|Enum|Equal(Enum) Command "NewEnumerator0") (Utilities|Enum|Equal(Enum) Command "NewEnumerator1") (Utilities|Enum|Equal(Enum) Command "NewEnumerator2") (Utilities|Enum|Equal(Enum) Command "NewEnumerator3"))))

(fn RoomWalk
  (params (Location :type Vector))
  ;[1 1 1] Work out the room ID when the player walks into a new room
  (bind _values (Utilities|Map|Values (LocalVariables|GetRoom%20Locations_0)))
  (for (_array_element _array_index) _values
    (if (and (Math|Float|NearlyEqual(Float) (.x _array_element) (.x Location) 5e+02) (Math|Float|NearlyEqual(Float) (.y _array_element) (.y Location) 5e+02))
      (bind _returnvalue (Actor|GetActorOfClass 0 "/Game/Blueprints/Zombie_BP.Zombie_BP_C"))
      (Variables|/Game/Blueprints/Zombie_BP.Zombie_BP_C|SetZombie%20Dead? _returnvalue false)
      (return _array_index))))