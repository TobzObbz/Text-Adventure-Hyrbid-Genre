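; Interactable chest that gives the first-person character a health potion.
; A box overlap enables input and shows the interact prompt; leaving disables input and replaces all widgets with the movement HUD.
; Interact first plays a timeline rotating the lid open, then a later press increments the potion count, updates a newly created HUD widget and destroys the chest.
; ResetChest only stores the passed chest reference.
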(event OnComponentBeginOverlap(Box)
  (params (OverlappedComponent :type Primitive%20Component%20Object%20Reference) (OtherActor :type Actor%20Object%20Reference) (OtherComp :type Primitive%20Component%20Object%20Reference) (OtherBodyIndex :type Integer) (bFromSweep :type Boolean) (SweepResult :type Hit%20Result%20Structure%20%28by%20ref%29))
  (Utilities|Casting|CastToBP_FirstPersonCharacter OtherActor)
  (Variables|Default|SetIn%20Collision? true)
  (Input|EnableInput (Game|GetPlayerController 0))
  (bind _returnvalue (UserInterface|CreateWidget "/Game/UI/PressEToInteract_UI.PressEToInteract_UI_C"))
  (UserInterface|Viewport|AddtoViewport _returnvalue 0))

(event OnComponentEndOverlap(Box)
  (params (OverlappedComponent :type Primitive%20Component%20Object%20Reference) (OtherActor :type Actor%20Object%20Reference) (OtherComp :type Primitive%20Component%20Object%20Reference) (OtherBodyIndex :type Integer))
  (Utilities|Casting|CastToBP_FirstPersonCharacter OtherActor)
  (Variables|Default|SetIn%20Collision? false)
  (Input|DisableInput (Game|GetPlayerController 0))
  (Viewport|RemoveAllWidgets)
  (bind _returnvalue (UserInterface|CreateWidget "/Game/UI/MovementVisualAdventure_UI.MovementVisualAdventure_UI_C"))
  (UserInterface|Viewport|AddtoViewport _returnvalue 0))

(event Custom|Reset%20Chest
  (params (Chest :type Map%20of%20Integers%20to%20Booleans))
  ;[1 1 1] Reset Chest
  (Variables|Default|SetChest_0 Chest))

(event Input|ActionEvents|InputActionInteract
  (params (Key :type Key%20Structure :default "None"))
  (:Pressed
    (if (Variables|Default|GetOpen?)
      (bind _asbp_first_person_character (Utilities|Casting|CastToBP_FirstPersonCharacter (Game|GetPlayerCharacter 0)))
      (bind _result (Math|Integer|IncrementInt (Variables|/Game/FirstPerson/Blueprints/BP_FirstPersonCharacter.BP_FirstPersonCharacter_C|GetHealth%20Potions _asbp_first_person_character))
        (:%20%20
          (bind _output_get (Variables|/Game/FirstPerson/Blueprints/BP_FirstPersonCharacter.BP_FirstPersonCharacter_C|SetHealth%20Potions _asbp_first_person_character _result))
          (Components|DestroyComponent (Variables|Default|GetHealth%20Potion))
          (bind _returnvalue (UserInterface|CreateWidget "/Game/UI/MovementVisualAdventure_UI.MovementVisualAdventure_UI_C"))
          (Default|UpdateHealthPotion _returnvalue _output_get)
          (Actor|DestroyActor)))
      (elif (Variables|Default|GetIn%20Collision?)
        (bind _chest_open (Timeline|Open%20Chest PlayFromStart)
          (:Update
            (Transformation|SetRelativeRotation (Variables|Default|GetScene) (Math|Rotator|Lerp(Rotator) "0, 0, 0" "50.000000,0.000000,0.000000" _chest_open) false false))
          (:Finished
            (Variables|Default|SetOpen? true)))))))

(fn ConstructionScript)