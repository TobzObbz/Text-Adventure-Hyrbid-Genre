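; Room actor whose trigger box drives a room-based adventure UI once the first-person character reaches a minimum Stage.
; On overlap, RoomWalk turns the player's location into a room ID.
; Special IDs show a win screen then the title screen, or the player UI while setting FinalWidget, which blocks further adventure UI rebuilds that otherwise carry the room ID and stage rule.
; The construction script picks the straight, corner, dead-end or T mesh from RoomType.
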(event OnComponentBeginOverlap(Box)
  (params (OverlappedComponent :type Primitive%20Component%20Object%20Reference) (OtherActor :type Actor%20Object%20Reference) (OtherComp :type Primitive%20Component%20Object%20Reference) (OtherBodyIndex :type Integer) (bFromSweep :type Boolean) (SweepResult :type Hit%20Result%20Structure%20%28by%20ref%29))
  (bind _asbp_first_person_character (Utilities|Casting|CastToBP_FirstPersonCharacter OtherActor))
  (if (>= (Variables|/Game/FirstPerson/Blueprints/BP_FirstPersonCharacter.BP_FirstPersonCharacter_C|GetStage? _asbp_first_person_character) 7)
    (bind _asbp_first_person_character_2 (Utilities|Casting|CastToBP_FirstPersonCharacter (Game|GetPlayerCharacter 0)))
    (bind _new_room_id (CallFunction|RoomWalk (Transformation|GetActorLocation _asbp_first_person_character_2)))
    (bind _output_get (Variables|Default|SetRoomID _new_room_id))
    (bind _returnvalue (UserInterface|CreateWidget "/Game/UI/MovementVisualAdventure_UI.MovementVisualAdventure_UI_C"))
    (if (>= (Variables|/Game/UI/MovementVisualAdventure_UI.MovementVisualAdventure_UI_C|GetStage _returnvalue) 9)
      (bind _returnvalue_2 (UserInterface|CreateWidget "/Game/UI/Player_UI.Player_UI_C"))
      (UserInterface|Viewport|AddtoViewport _returnvalue_2 0))
    (if (== _output_get 15)
      (bind _returnvalue_3 (UserInterface|CreateWidget "/Game/UI/YouWin_UI.YouWin_UI_C"))
      (UserInterface|Viewport|AddtoViewport _returnvalue_3 0)
      (Utilities|FlowControl|Delay 2.0)
      (Viewport|RemoveAllWidgets)
      (bind _returnvalue_4 (UserInterface|CreateWidget "/Game/UI/TitleScreen_UI.TitleScreen_UI_C"))
      (UserInterface|Viewport|AddtoViewport _returnvalue_4 0)
      (elif (== _output_get 14)
        (Viewport|RemoveAllWidgets)
        (bind _returnvalue_5 (UserInterface|CreateWidget "/Game/UI/Player_UI.Player_UI_C"))
        (UserInterface|Viewport|AddtoViewport _returnvalue_5 0)
        (bind _asbp_first_person_character_3 (Utilities|Casting|CastToBP_FirstPersonCharacter (Game|GetPlayerCharacter 0)))
        (Variables|/Game/FirstPerson/Blueprints/BP_FirstPersonCharacter.BP_FirstPersonCharacter_C|SetFinal%20Widget? _asbp_first_person_character_3 true)
        (elif (not (Variables|/Game/FirstPerson/Blueprints/BP_FirstPersonCharacter.BP_FirstPersonCharacter_C|GetFinal%20Widget? (.AsBP%20First%20Person%20Character (Utilities|Casting|CastToBP_FirstPersonCharacter (Game|GetPlayerCharacter 0)))))
          (Viewport|RemoveAllWidgets)
          (bind _returnvalue_6 (UserInterface|CreateWidget "/Game/UI/MovementVisualAdventure_UI.MovementVisualAdventure_UI_C"))
          (Default|SetCurrentRoomID _returnvalue_6 _output_get)
          (Default|ChangeRule _returnvalue_6 (Variables|/Game/UI/MovementVisualAdventure_UI.MovementVisualAdventure_UI_C|GetStage _returnvalue))
          (UserInterface|Viewport|AddtoViewport _returnvalue_6 0))))))

(fn ConstructionScript
  (Components|StaticMesh|SetStaticMesh (Variables|Default|GetStaticMesh) (Utilities|Select :Index (Variables|Default|GetRoom%20Type) :NewEnumerator0 "/Game/Assets/Rooms/Straight_Room/Straight_Room.Straight_Room" :NewEnumerator1 "/Game/Assets/Rooms/Corner_Room/Corner_Room.Corner_Room" :NewEnumerator2 "/Game/Assets/Rooms/Dead_End_Room/Dead_End_Room.Dead_End_Room" :NewEnumerator3 "/Game/Assets/Rooms/T_Room/T_Room.T_Room")))