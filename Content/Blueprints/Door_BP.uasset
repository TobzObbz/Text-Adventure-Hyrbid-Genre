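; Door_BP is a sliding door that opens while the first-person character is inside its Box trigger and closes when they leave.
; OpenDoor plays the DoorMove timeline from the start to lerp the mesh sideways along Y, and CloseDoor reverses it from the end.
; A separate OpenClose event opens the door, waits briefly, then closes it.
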(event OnComponentBeginOverlap(Box)
  (params (OverlappedComponent :type Primitive%20Component%20Object%20Reference) (OtherActor :type Actor%20Object%20Reference) (OtherComp :type Primitive%20Component%20Object%20Reference) (OtherBodyIndex :type Integer) (bFromSweep :type Boolean) (SweepResult :type Hit%20Result%20Structure%20%28by%20ref%29))
  (Utilities|Casting|CastToBP_FirstPersonCharacter OtherActor)
  (CallFunction|OpenDoor))

(event OnComponentEndOverlap(Box)
  (params (OverlappedComponent :type Primitive%20Component%20Object%20Reference) (OtherActor :type Actor%20Object%20Reference) (OtherComp :type Primitive%20Component%20Object%20Reference) (OtherBodyIndex :type Integer))
  (Utilities|Casting|CastToBP_FirstPersonCharacter OtherActor)
  (CallFunction|CloseDoor))

(event Custom|Open%20Door
  (bind _door_movement (Timeline|Door%20Move PlayFromStart)
    (:Update
      (Transformation|SetRelativeLocation (Variables|Default|GetStaticMesh) (Math|Vector|Lerp(Vector) "0, 0, 0" "0,150.000000, 0" _door_movement) false false))))

(event Custom|Close%20Door
  (bind _door_movement (Timeline|Door%20Move ReverseFromEnd)
    (:Update
      (Transformation|SetRelativeLocation (Variables|Default|GetStaticMesh) (Math|Vector|Lerp(Vector) "0, 0, 0" "0,150.000000, 0" _door_movement) false false))))

(event Custom|OpenClose
  (CallFunction|OpenDoor)
  (Utilities|FlowControl|Delay 0.5)
  (CallFunction|CloseDoor))

(fn ConstructionScript)