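; Zombie Blueprint that runs combat between zombies and the first-person player, tracking zombie presence per room in a map.
; If the current room holds a zombie, an attack sets a punch flag and deals random damage to player health, showing the death screen at zero.
; Player hits subtract random damage from zombie health, flag death and restore health after a delay.
; Separate events clear a room's zombie or reset the whole map.
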(event Custom|Zombie%20Attack
  (params (Current%20Room%20ID :type Integer))
  ;[1 1 1] Zombie attacks the player
  (bind _values (Utilities|Map|Values (Variables|Default|GetZombie)))
  (if (Utilities|Array|Get(acopy) _values Current%20Room%20ID)
    (Variables|Default|SetZombie%20Punch true)
    (bind _output_get (Variables|Default|SetZombie%20Damage (Math|Random|RandomIntegerinRange 2 5)))
    (bind _asbp_first_person_character (Utilities|Casting|CastToBP_FirstPersonCharacter (Game|GetPlayerCharacter 0)))
    (bind _output_get_2 (Variables|/Game/FirstPerson/Blueprints/BP_FirstPersonCharacter.BP_FirstPersonCharacter_C|SetHealth _asbp_first_person_character (- (Variables|/Game/FirstPerson/Blueprints/BP_FirstPersonCharacter.BP_FirstPersonCharacter_C|GetHealth _asbp_first_person_character) _output_get)))
    (if (<= _output_get_2 0.0)
      (Viewport|RemoveAllWidgets)
      (bind _returnvalue (UserInterface|CreateWidget "/Game/UI/YouDie_UI.YouDie_UI_C"))
      (UserInterface|Viewport|AddtoViewport _returnvalue 0))
    (else
      (Variables|Default|SetZombie%20Punch false))))

(event Custom|Remove%20Zombie
  (params (Room%20Index :type Integer))
  ;[1 1 1] Remove zombie from map
  (Utilities|Map|Add (Variables|Default|GetZombie) Room%20Index false))

(event Custom|Attack%20Zombie
  ;[1 1 1] Player attacks the zombie
  (bind _output_get (Variables|Default|SetAttack%20Damage (Math|Random|RandomIntegerinRange 2 10)))
  (bind _output_get_2 (Variables|Default|SetZombie%20Health (- (Variables|Default|GetZombie%20Health) _output_get)))
  (if (<= _output_get_2 0.0)
    (Variables|Default|SetZombie%20Dead? true)
    (Utilities|FlowControl|Delay 4.38)
    (Variables|Default|SetZombie%20Health 1e+01)
    (else
      (Variables|Default|SetZombie%20Dead? false))))

(event Custom|Reset%20Zombies
  (params (Zombies :type Map%20of%20Integers%20to%20Booleans))
  ;[1 1 1] Reset Zombies
  (Variables|Default|SetZombie Zombies))

(fn ConstructionScript)